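; Base weapon Blueprint that handles firing, reloading and ammo for its owning character through an EBBarrel ballistics component.
; StartShoot and StopShoot drive the barrel, whose shot-fired event plays the owner's fire montage, muzzle flash, trace and sound.
; StartReload blocks shooting and plays reload feedback, then a separately called EndReload moves reserve ammo into the magazine.
; UpdateBarrelLocation is an empty hook called while shooting, and Tick draws optional muzzle-to-barrel debug shapes.
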(event Custom|StartShoot
  ;[1 1 1] Start And Stop Shoot Event
  (if (not (Variables|/Script/EasyBallistics.EBBarrel|GetShootingBlocked (Variables|Default|GetEBBarrel)))
    (Variables|Default|SetbIsShooting true)
    (CallFunction|UpdateBarrelLocation)
    (Class|EBBarrel|Shoot (Variables|Default|GetEBBarrel) true)))

(event Custom|StopShoot
  ;[1 1 1] Start And Stop Shoot Event
  (Variables|Default|SetbIsShooting false)
  (Class|EBBarrel|Shoot (Variables|Default|GetEBBarrel) false)
  (Transformation|SetWorldTransform (Variables|Default|GetEBBarrel) (Transformation|GetWorldTransform (Variables|Default|GetMuzzleFlash)) false false))

(event Custom|OnShotFired
  ;[1 1 1] EventsOnShoot
  (Animation|PlayAnimMontage (Variables|Default|GetWeaponOwnerRef) (Variables|Default|GetCharacterFireMontage) 1.0 "None")
  (Effects|SpawnEmitterAttached (Variables|Default|GetWeaponMuzzleFlash) (Variables|Default|GetMuzzleLocation) "None")
  (Effects|SpawnEmitterAttached (Variables|Default|GetWeaponTrace) (Variables|Default|GetTrace) "None")
  (Audio|SpawnSoundAttached (Variables|Default|GetWeaponFireSound) (Variables|Default|GetMuzzleLocation) "None" "0, 0, 0" "0, 0, 0" "KeepRelativeOffset" false 1.0 1.0 0.0 0 0))

(event EventBeginPlay
  (Variables|Default|SetCurrentRemainingAmmo (Variables|Default|GetMaxRemainingAmmo))
  ;[1 1 1] EventsOnShoot
  (EventDispatchers|BindEventtoShotFired (Variables|Default|GetEBBarrel) (delegate Custom|OnShotFired)))

(event EventTick
  (params (DeltaSeconds :type Float%20%28single-precision%29))
  (Debug|DebugDraw)
  (if (Variables|Default|GetbIsShooting)
    (CallFunction|UpdateBarrelLocation)
    (if true
      _)))

(fn ConstructionScript)

(fn DebugDraw
  (bind _muzzlelocation (Variables|Default|GetMuzzleLocation))
  (bind _ebbarrel (Variables|Default|GetEBBarrel))
  (bind _returnvalue (Transformation|GetWorldLocation _ebbarrel))
  (bind _returnvalue_2 (Transformation|GetWorldLocation _muzzlelocation))
  (if (Variables|Default|GetbEnableDebug)
    (Rendering|Debug|DrawDebugLine _returnvalue_2 _returnvalue "(R=0.484375,G=0.019497,B=0.043600,A=1.000000)" 0.0 2.0)
    (Rendering|Debug|DrawDebugSphere _returnvalue_2 2e+01 12 "(R=0.828842,G=0.838542,B=0.017284,A=1.000000)" 0.0)
    (Rendering|Debug|DrawDebugSphere _returnvalue 2e+01 12 "(R=0.157171,G=0.226845,B=0.838542,A=1.000000)" 0.0)))

(fn StartReload
  (if (not (Variables|Default|GetbIsReloading))
    (if (> (Variables|Default|GetCurrentRemainingAmmo) 0)
      (Ammo|GetRequiredAmmo)
      (if (not (== (Variables|Default|GetRequiredAmmoCount) 0))
        (Variables|/Script/EasyBallistics.EBBarrel|SetShootingBlocked (Variables|Default|GetEBBarrel) true)
        (Variables|Default|SetbIsReloading true)
        (Animation|PlayAnimMontage (Variables|Default|GetWeaponOwnerRef) (Variables|Default|GetCharacterReloadMontage) 1.0 "None")
        (Audio|Components|Audio|Play (Variables|Default|GetReload%20Sound) 0.0)))))

(fn GetRequiredAmmo
  (bind _magazinesize (Variables|Default|GetMagazineSize))
  (Variables|Default|SetRequiredAmmoCount (Math|Integer|Clamp(Integer) (- _magazinesize (Class|EBBarrel|GetAmmoCount (Variables|Default|GetEBBarrel) true)) 0 _magazinesize)))

(fn GetCurrentRemainingAmmo
  (return (Variables|Default|GetCurrentRemainingAmmo)))

(fn GetCurrentMagazineAmmo
  (return (Class|EBBarrel|GetAmmoCount (Variables|Default|GetEBBarrel) true)))

(fn UpdateBarrelLocation)

(fn EndReload
  (bind _ebbarrel (Variables|Default|GetEBBarrel))
  (bind _ebbarrel_2 (Variables|Default|GetEBBarrel))
  (if (< (Variables|Default|GetRequiredAmmoCount) (Variables|Default|GetCurrentRemainingAmmo))
    (Variables|Default|SetCurrentRemainingAmmo (- (Variables|Default|GetCurrentRemainingAmmo) (Variables|Default|GetRequiredAmmoCount)))
    (Class|EBBarrel|SetAmmo _ebbarrel_2 (+ (Class|EBBarrel|GetAmmoCount (Variables|Default|GetEBBarrel) true) (Variables|Default|GetRequiredAmmoCount)) true false false (Class|EBBarrel|GetAmmo _ebbarrel_2 true))
    (else
      (Class|EBBarrel|SetAmmo _ebbarrel (+ (Class|EBBarrel|GetAmmoCount (Variables|Default|GetEBBarrel) true) (Variables|Default|GetCurrentRemainingAmmo)) true false false (Class|EBBarrel|GetAmmo _ebbarrel true))
      (Variables|Default|SetCurrentRemainingAmmo 0)))
  (Variables|/Script/EasyBallistics.EBBarrel|SetShootingBlocked (Variables|Default|GetEBBarrel) false)
  (Variables|Default|SetbIsReloading false)
  (Development|PrintString "Reload is Done"))